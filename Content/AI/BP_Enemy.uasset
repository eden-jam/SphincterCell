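; Enemy AI character for a top-down stealth-style game that triggers a loss once it spots the player.
; Each tick a fan of line traces builds a vision cone, drawn as canvas triangles into a render target feeding a dynamic material on its plane.
; A trace hitting the player sets SeenPlayer, which calls OnLoose on the game mode.
; Overlapping a "Fart"-tagged actor kills it: it ragdolls, sets HasFart and decrements the alive count it incremented on BeginPlay.
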(event `self.ReceiveTick`
  (params (DeltaSeconds :type "Float (single-precision)"))
  (if (`self.IsAlive`)
    (`|ExecutionSequence`
      (:`then_0`
        (`self.LosVisionSystem`))
      (:`then_1`
        (if (`KismetSystemLibrary.IsValid` (`self.SeenPlayer`))
          (bind _outactors (`GameplayStatics.GetAllActorsOfClass` "/Game/TopDown/Blueprints/BP_TopDownGameMode.BP_TopDownGameMode_C"))
          (`/Game/TopDown/Blueprints/BP_TopDownGameMode.OnLoose` (`|GetArrayItem` _outactors)))))))

(event `self.CapsuleComponent.OnComponentBeginOverlap`
  (params (OverlappedComponent :type "PrimitiveComponent Object Reference") (OtherActor :type "Actor Object Reference") (OtherComp :type "PrimitiveComponent Object Reference") (OtherBodyIndex :type Integer) (bFromSweep :type Boolean) (SweepResult :type "HitResult Structure (by ref)"))
  (`KismetSystemLibrary.PrintString` (`KismetSystemLibrary.GetDisplayName` OtherActor))
  (if (and (`self.IsAlive`) (`self.ActorHasTag` OtherActor "Fart"))
    (`self.OnKilled`)
    (set `self.IsAlive` false)))

(event `OnKilled`
  (bind _asmy_game_instance (cast `/Game/Game/MyGameInstance` (`GameplayStatics.GetGameInstance`)))
  (set `/Game/Game/MyGameInstance.HasFart` true _asmy_game_instance)
  (bind _asbp_top_down_game_mode (cast `/Game/TopDown/Blueprints/BP_TopDownGameMode` (`GameplayStatics.GetGameMode`)))
  (bind _output_get (set `/Game/TopDown/Blueprints/BP_TopDownGameMode.AmountAlive` (- (`/Game/TopDown/Blueprints/BP_TopDownGameMode.AmountAlive` _asbp_top_down_game_mode) 1) _asbp_top_down_game_mode))
  (`|ExecutionSequence`
    (:`then_0`
      (`PrimitiveComponent.SetSimulatePhysics` (`self.Mesh`) true)
      (`CharacterMovementComponent.DisableMovement` (`self.CharacterMovement`))
      (`PrimitiveComponent.SetCollisionEnabled` (`self.CapsuleComponent`) "NoCollision"))
    (:`then_1`
      (`KismetSystemLibrary.PrintString` (`KismetStringLibrary.Conv_IntToString` _output_get)))))

(event `self.ReceiveBeginPlay`
  (`|ExecutionSequence`
    (:`then_0`
      (bind _returnvalue (`KismetRenderingLibrary.CreateRenderTarget2D` 1800 1800))
      (set `self.LosRenderTarget` _returnvalue))
    (:`then_1`
      (bind _returnvalue_2 (`PrimitiveComponent.CreateDynamicMaterialInstance` (`self.Plane`) 0 "/Game/AI/VisionCone/LosVisionMat.LosVisionMat" "None"))
      (set `self.DynamicMaterial` _returnvalue_2))
    (:`then_2`
      ;[1 1 1] Comment
      (bind _asbp_top_down_game_mode (cast `/Game/TopDown/Blueprints/BP_TopDownGameMode` (`GameplayStatics.GetGameMode`)))
      (bind _output_get (set `/Game/TopDown/Blueprints/BP_TopDownGameMode.AmountAlive` (+ (`/Game/TopDown/Blueprints/BP_TopDownGameMode.AmountAlive` _asbp_top_down_game_mode) 1) _asbp_top_down_game_mode))
      (`KismetSystemLibrary.PrintString` (`KismetStringLibrary.Conv_IntToString` _output_get)))))

(fn `CreateCone`
  (bind _returnvalue (`self.K2_GetActorLocation`))
  (bind _traceresults (`self.TraceResults`))
  (`KismetArrayLibrary.Array_Clear` (`self.TraceResults`))
  (for _index (range (+ (`self.NumTraces`) 1))
    (bind _returnvalue_2 (+ (* (`KismetMathLibrary.GreaterGreater_VectorRotator` (`KismetMathLibrary.GreaterGreater_VectorRotator` (`self.GetActorForwardVector`) (`KismetMathLibrary.MakeRotator` 0.0 0.0 (/ (* (`self.NumTraces`) (`self.DegreePreTrace`)) -2.0))) (`KismetMathLibrary.MakeRotator` 0.0 0.0 (* (`self.DegreePreTrace`) _index))) 700.0) _returnvalue))
    (bind (_outhit _returnvalue_3) (`KismetSystemLibrary.LineTraceSingleForObjects` :`Start` _returnvalue :`End` _returnvalue_2 :`ObjectTypes` (`|MakeArray` "ObjectTypeQuery3" "ObjectTypeQuery1" "ObjectTypeQuery2" "ObjectTypeQuery4" :!type "EObjectTypeQuery Enum") :`DrawDebugType` "ForOneFrame"))
    (if _returnvalue_3
      (bind (_bblockinghit _binitialoverlap _time _distance _location _impactpoint _normal _impactnormal _physmat _hitactor) (`GameplayStatics.BreakHitResult` _outhit))
      (`KismetArrayLibrary.Array_Add` _traceresults _impactpoint)
      (bind _asbp_top_down_character (cast `/Game/TopDown/Blueprints/BP_TopDownCharacter` _hitactor))
      (set `self.SeenPlayer` _asbp_top_down_character)
      (else
        (`KismetArrayLibrary.Array_Add` _traceresults _returnvalue_2)))))

(fn `LosVisionSystem`
  (bind _losrendertarget (`self.LosRenderTarget`))
  (`|ExecutionSequence`
    (:`then_0`
      (`self.CreateCone`))
    (:`then_1`
      (`self.PrepareTriangles`))
    (:`then_2`
      (`KismetRenderingLibrary.ClearRenderTarget2D` _losrendertarget)
      (bind (_canvas _size _context) (`KismetRenderingLibrary.BeginDrawCanvasToRenderTarget` _losrendertarget))
      (`Canvas.K2_DrawTriangle` _canvas null (`self.CanvasTriangles`))
      (`MaterialInstanceDynamic.SetTextureParameterValue` (`self.DynamicMaterial`) "MainTexture" _losrendertarget)
      (`KismetRenderingLibrary.EndDrawCanvasToRenderTarget` _context))))

(fn `PrepareTriangles`
  (bind _returnvalue (`self.K2_GetActorLocation`))
  (bind _returnvalue_2 (`KismetMathLibrary.MakeVector` 900.0 900.0))
  (`KismetArrayLibrary.Array_Clear` (`self.CanvasTriangles`))
  (for _index (range (+ (- (`KismetArrayLibrary.Array_Length` (`self.TraceResults`)) 2) 1))
    (`KismetArrayLibrary.Array_Add` (`self.CanvasTriangles`) (make `CanvasUVTri` (`KismetMathLibrary.Conv_VectorToVector2D` _returnvalue_2) (0.0 0.0) (struct :`R` 1.0 :`G` 1.0 :`B` 1.0) (`KismetMathLibrary.Conv_VectorToVector2D` (+ (- (`|GetArrayItem` (`self.TraceResults`) _index) _returnvalue) _returnvalue_2)) (0.0 0.0) (struct :`R` 1.0 :`G` 1.0 :`B` 1.0) (`KismetMathLibrary.Conv_VectorToVector2D` (+ (- (`|GetArrayItem` (`self.TraceResults`) (+ _index 1)) _returnvalue) _returnvalue_2)) (0.0 0.0) (struct :`R` 1.0 :`G` 1.0 :`B` 1.0)))))

(fn `UserConstructionScript`)