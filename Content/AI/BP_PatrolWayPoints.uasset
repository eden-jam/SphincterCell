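; BP_PatrolWayPoints holds an ordered list of AI patrol waypoints and tracks the current one.
; BeginPlay sets CurrentWayPoint to the first entry in the WayPoints array.
; SetNextWayPoint looks up the current entry's index and advances it by one, using modulo on the array length to loop back to the start.
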(event `self.ReceiveBeginPlay`
  (set `self.CurrentWayPoint` (`|GetArrayItem` (`self.WayPoints`))))

(fn `SetNextWayPoint`
  (bind _waypoints (`self.WayPoints`))
  (set `self.CurrentWayPoint` (`|GetArrayItem` _waypoints (mod (+ (`KismetArrayLibrary.Array_Find` _waypoints (`self.CurrentWayPoint`)) 1) (`KismetArrayLibrary.Array_Length` _waypoints)))))